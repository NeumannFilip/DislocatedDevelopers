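; BP_DefaultItem is an item actor with collection reporting for the quest system.
; NotifyCollected gets the current quest from BP_TestGameModeBase and calls UpdateObjective on each objective whose ItemToCollect class the item matches or derives from.
; InteractionBox and StaticMesh overlap events only cast to FirstPersonCharacterTest, with nothing following.
; The NotifyCollected call and BW_EquipItem widget nodes in this graph are disconnected.
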(event `self.InteractionBox.OnComponentBeginOverlap`
  (params (OverlappedComponent :type "PrimitiveComponent Object Reference") (OtherActor :type "Actor Object Reference") (OtherComp :type "PrimitiveComponent Object Reference") (OtherBodyIndex :type Integer) (bFromSweep :type Boolean) (SweepResult :type "HitResult Structure (by ref)"))
  (cast `FirstPersonCharacterTest` OtherActor))

(event `self.InteractionBox.OnComponentEndOverlap`
  (params (OverlappedComponent :type "PrimitiveComponent Object Reference") (OtherActor :type "Actor Object Reference") (OtherComp :type "PrimitiveComponent Object Reference") (OtherBodyIndex :type Integer))
  (cast `FirstPersonCharacterTest` OtherActor))

(event `Event Notify Collected`
  (bind _asbp_test_game_mode_base (cast `/Game/GameState/BP_TestGameModeBase` (`GameplayStatics.GetGameMode`)))
  (bind _currentquestreference (`/Game/GameState/BP_TestGameModeBase.CurrentQuestReference` _asbp_test_game_mode_base))
  (for _array_element (`TestQuest.objectives` _currentquestreference)
    (bind (_cleartype _itemtocollect _description _objectiveid) (break `Objective` _array_element))
    (if (`KismetMathLibrary.ClassIsChildOf` (`GameplayStatics.GetObjectClass` self) _itemtocollect)
      (`TestQuest.UpdateObjective` _currentquestreference _objectiveid 0))))

(event `self.StaticMesh.OnComponentBeginOverlap`
  (params (OverlappedComponent :type "PrimitiveComponent Object Reference") (OtherActor :type "Actor Object Reference") (OtherComp :type "PrimitiveComponent Object Reference") (OtherBodyIndex :type Integer) (bFromSweep :type Boolean) (SweepResult :type "HitResult Structure (by ref)"))
  (cast `FirstPersonCharacterTest` OtherActor))

(fn `UserConstructionScript`)