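; BP_NPCOld is a quest-system NPC that walks a looping route and can be talked to by the player.
; Interaction calls Focus(false) on the player and begins its Dialogue through the player's Narrative component, passing player character 0 as the NPC.
; Finishing interaction resets the player camera's field of view.
; From BeginPlay, AIMoveTo cycles through the Destinations actors, advancing only on success, with no failure handling.
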(event `/Game/QuestSystem/BI_Interaction.OnInteraction`
  (params (PlayerCharacter :type "/Game/FirstPerson/Blueprints/BP_FirstPersonCharacter Object Reference"))
  (bind _returnvalue (`NarrativeFunctionLibrary.GetNarrativeComponentFromTarget` PlayerCharacter))
  (`/Game/FirstPerson/Blueprints/BP_FirstPersonCharacter.Focus` PlayerCharacter false)
  (`/Engine/EditorBlueprintResources/StandardMacros.IsValid` _returnvalue
    (:`Is Valid`
      (`NarrativeComponent.BeginDialogue` _returnvalue (`self.Dialogue`) (`GameplayStatics.GetPlayerCharacter` 0) "None"))))

(event `/Game/QuestSystem/BI_Interaction.OnInteractionFinish`
  (params (PlayerCharacter :type "/Game/FirstPerson/Blueprints/BP_FirstPersonCharacter Object Reference"))
  (`CameraComponent.SetFieldOfView` (`Game3Character.FirstPersonCameraComponent` PlayerCharacter) 90.0))

(event `MoveToTarget`)

(event `self.ReceiveBeginPlay`
  (bind _returnvalue (+ (`self.Target`) 1))
  (if true
    (`|AIMoveTo` (`self.GetController`) null (0.0 0.0 0.0) (`|GetArrayItem` (`self.Destinations`) (`self.Target`)) :!label _label
      (:`OnSuccess`
        (if (== _returnvalue (`KismetArrayLibrary.Array_Length` (`self.Destinations`)))
          (set `self.Target` 0)
          (goto _label)
          (else
            (set `self.Target` _returnvalue)
            (goto _label)))))))

(fn `UserConstructionScript`)