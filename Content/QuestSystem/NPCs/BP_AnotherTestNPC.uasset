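; BP_AnotherTestNPC is a quest system test NPC that patrols a looping list of destination actors.
; MoveToTarget checks the State enum once, then chains AI MoveTo calls, advancing the target index on each success and wrapping to the first.
; The loop does not recheck State and has no failure handling; BeginPlay is empty, so MoveToTarget needs an outside trigger.
; UpdateWalkSpeed sets the movement component's max walk speed.
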(event `MoveToTarget`
  (bind _returnvalue (+ (`self.Target`) 1))
  (if (`|EnumEquality` (`self.State`) "NewEnumerator0")
    (`|AIMoveTo` (`self.GetController`) null (0.0 0.0 0.0) (`|GetArrayItem` (`self.Destinations`) (`self.Target`)) :!label _label
      (:`OnSuccess`
        (if (== _returnvalue (`KismetArrayLibrary.Array_Length` (`self.Destinations`)))
          (set `self.Target` 0)
          (goto _label)
          (else
            (set `self.Target` _returnvalue)
            (goto _label)))))))

(event `self.ReceiveBeginPlay`)

(fn `UpdateWalkSpeed`
  (params (NewWalkSpeed :type "Float (double-precision)"))
  (set `CharacterMovementComponent.MaxWalkSpeed` NewWalkSpeed (`self.CharacterMovement`)))

(fn `UserConstructionScript`)