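; Test game mode that puts a heads-up display item widget on screen at BeginPlay and holds prototype quest HUD logic.
; A disconnected chain builds a player HUD and tutorial quest with objective widgets, so the HUD and quest references are never set here.
; HideQuest removes the quest panel, while HideObjective only creates an unattached copy of the matching objective widget without hiding it.
; UpdateObjectiveHUD is an empty stub.
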(event `self.ReceiveBeginPlay`
  (bind _returnvalue (`|CreateWidget` "/Game/GrabAndInspect/BW_HeadsUpDisplayItem.BW_HeadsUpDisplayItem_C"))
  (bind _output_get (set `self.HeadsUpDisplay` _returnvalue))
  (`UserWidget.AddToViewport` _output_get 0))

(event `self.UpdateObjectiveHUD`
  (params (_objectiveNum :type Integer)))

(event `self.HideObjective`
  (params (_objectiveNum :type Integer))
  (bind (_cleartype _itemtocollect _description _objectiveid) (break `Objective` (`|GetArrayItem` (`TestQuest.objectives` (`self.CurrentQuestReference`)) _objectiveNum)))
  (for _array_element (`PanelWidget.GetAllChildren` (`/Game/Player/BW_PlayerHUD.ObjectiveVerticalBox` (`self.HUD Reference`)))
    (bind _asbw_objective_info (cast `/Game/Player/BW_ObjectiveInfo` _array_element))
    (if (== (`/Game/Player/BW_ObjectiveInfo.Objective ID` _asbw_objective_info) _objectiveNum)
      (bind _returnvalue (`|CreateWidget` "/Game/Player/BW_ObjectiveInfo.BW_ObjectiveInfo_C"))
      (`/Game/Player/BW_ObjectiveInfo.SetObjectiveID` _returnvalue _objectiveid)
      (`/Game/Player/BW_ObjectiveInfo.SetObjectiveDescriptionText` _returnvalue (`KismetTextLibrary.Conv_StringToText` _description)))))

(event `self.HideQuest`
  (`Widget.RemoveFromParent` (`/Game/Player/BW_PlayerHUD.BW_QuestInfo` (`self.HUD Reference`))))

(fn `UserConstructionScript`)