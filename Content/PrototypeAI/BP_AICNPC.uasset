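; AI controller for a prototype NPC that runs the BT_MoveTo behavior tree on possess and tracks the player through AI perception.
; Successfully sensing a Player-tagged actor cancels the timer and writes that actor and an in-sight flag to the Blackboard.
; Any other perception update starts a LineOfSight-length timer that clears both keys on expiry, giving a grace period before the player is forgotten.
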(event `self.ReceivePossess`
  (params (PossessedPawn :type "Pawn Object Reference"))
  (`self.RunBehaviorTree` "/Game/PrototypeAI/BT_MoveTo.BT_MoveTo"))

(event `self.AIPerception.OnTargetPerceptionUpdated`
  (params (Actor :type "Actor Object Reference") (Stimulus :type "AIStimulus Structure"))
  (bind _blackboard (`self.Blackboard`))
  (if (and (`.bSuccessfullySensed` (break `AIStimulus` Stimulus)) (`self.ActorHasTag` Actor "Player"))
    (`KismetSystemLibrary.K2_ClearAndInvalidateTimerHandle` (`self.NPCTimer`))
    (`BlackboardComponent.SetValueAsBool` _blackboard (`self.Is Player In Sight`) true)
    (`BlackboardComponent.SetValueAsObject` _blackboard (`self.NPCActor`) Actor)
    (else
      (bind _returnvalue (`KismetSystemLibrary.K2_SetTimerDelegate` (delegate `StartNPCTimer`) (`self.Line Of Sight`)))
      (set `self.NPCTimer` _returnvalue))))

(event `StartNPCTimer`
  (bind _blackboard (`self.Blackboard`))
  (`BlackboardComponent.SetValueAsBool` _blackboard (`self.Is Player In Sight`) false)
  (`BlackboardComponent.SetValueAsObject` _blackboard (`self.NPCActor`) null))

(fn `UserConstructionScript`)