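; Base item actor that the player can pick up and inspect, showing a named pickup prompt when looked at.
; Interacting attaches it to the player's ItemGrip with physics and collision off, or starts inspection if an item is already held.
; Inspection hands input to the item, shows a description widget, and supports drag-to-rotate and wheel zoom along the camera's forward vector.
; InteractITem ends inspection; DropItem detaches it and restores physics.
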(event `/Game/GrabAndInspect/BI_InteractionInterface.LookAt`
  (params (PlayerCharacter :type "/Game/FirstPerson/Blueprints/BP_FirstPersonCharacter Object Reference"))
  (`/Game/GrabAndInspect/BW_HeadsUpDisplayItem.UpdateMessage` (`/Game/FirstPerson/Blueprints/BP_FirstPersonCharacter.HUD` PlayerCharacter) (`|FormatText` "Press E To Pick Up {name}" (`self.ItemName`))))

(event `/Game/GrabAndInspect/BI_InteractionInterface.InteractWith`
  (params (PlayerCharacter :type "/Game/FirstPerson/Blueprints/BP_FirstPersonCharacter Object Reference"))
  (bind _output_get (set `self.Player` PlayerCharacter))
  (`/Game/FirstPerson/Blueprints/BP_FirstPersonCharacter.Currently Held Item` _output_get
    (:`then`
      (`self.StartInspecting`))
    (:`else`
      (`self.PickUpItem`))))

(event `Key|LeftMouseButton`
  (params (Key :type "Key Structure"))
  (:`Pressed`
    (set `self.isRotating` true))
  (:`Released`
    (set `self.isRotating` false)))

(event `InputAxisKey|MouseX`
  (params (AxisValue :type "Float (single-precision)"))
  (if (`self.isRotating`)
    (`self.K2_SetActorRotation` (`KismetMathLibrary.ComposeRotators` (`self.K2_GetActorRotation`) (`KismetMathLibrary.MakeRotator` 0.0 0.0 (* AxisValue -5.0))))))

(event `InputAxisKey|MouseY`
  (params (AxisValue :type "Float (single-precision)"))
  (if (`self.isRotating`)
    (`self.K2_SetActorRotation` (`KismetMathLibrary.ComposeRotators` (`self.K2_GetActorRotation`) (`KismetMathLibrary.MakeRotator` 0.0 (* AxisValue -5.0))))))

(event `Key|MouseScrollUp`
  (params (Key :type "Key Structure"))
  (bind _returnvalue (`GameplayStatics.GetPlayerCameraManager` 0))
  (:`Pressed`
    (bind _output_get (set `self.Zooming` (`KismetMathLibrary.Clamp` (+ (`self.Zooming`) 1) 1 20)))
    (if (< _output_get 20)
      (`self.K2_SetActorLocation` (+ (`PlayerCameraManager.GetCameraLocation` _returnvalue) (* (`KismetMathLibrary.GetForwardVector` (`PlayerCameraManager.GetCameraRotation` _returnvalue)) (* (`self.Zooming`) 20)))))))

(event `Key|MouseScrollDown`
  (params (Key :type "Key Structure"))
  (bind _returnvalue (`GameplayStatics.GetPlayerCameraManager` 0))
  (:`Pressed`
    (bind _output_get (set `self.Zooming` (`KismetMathLibrary.Clamp` (- (`self.Zooming`) 1) 1 25)))
    (if (< _output_get 20)
      (`self.K2_SetActorLocation` (+ (`PlayerCameraManager.GetCameraLocation` _returnvalue) (* (`KismetMathLibrary.GetForwardVector` (`PlayerCameraManager.GetCameraRotation` _returnvalue)) (* (`self.Zooming`) 20)))))))

(event `InputAction|InteractITem`
  (params (Key :type "Key Structure"))
  (:`Pressed`
    (`self.StopInspecting`)))

(fn `DropItem`
  (bind _returnvalue (`GameplayStatics.GetPlayerCameraManager` 0))
  (`self.K2_DetachFromActor` "KeepWorld" "KeepWorld" "KeepWorld")
  (`self.K2_SetActorLocation` (+ (`PlayerCameraManager.GetCameraLocation` _returnvalue) (* (`KismetMathLibrary.GetForwardVector` (`PlayerCameraManager.GetCameraRotation` _returnvalue)) 200.0)))
  (`PrimitiveComponent.SetSimulatePhysics` (`self.StaticMesh`) true)
  (`PrimitiveComponent.SetCollisionEnabled` (`self.StaticMesh`) "QueryAndPhysics")
  (set `/Game/FirstPerson/Blueprints/BP_FirstPersonCharacter.Currently Held Item` self (`self.Player`)))

(fn `PickUpItem`
  (`self.K2_AttachToComponent` (`/Game/FirstPerson/Blueprints/BP_FirstPersonCharacter.ItemGrip` (`self.Player`)) "None" "SnapToTarget" "SnapToTarget" "KeepRelative")
  (`PrimitiveComponent.SetSimulatePhysics` (`self.StaticMesh`) false)
  (`PrimitiveComponent.SetCollisionEnabled` (`self.StaticMesh`) "NoCollision")
  (set `/Game/FirstPerson/Blueprints/BP_FirstPersonCharacter.Currently Held Item` self (`self.Player`)))

(fn `StartInspecting`
  (bind _returnvalue (`GameplayStatics.GetPlayerController` 0))
  (bind _returnvalue_2 (`GameplayStatics.GetPlayerCameraManager` 0))
  (`Widget.SetVisibility` (`/Game/FirstPerson/Blueprints/BP_FirstPersonCharacter.HUD` (`self.Player`)) "Hidden")
  (bind _returnvalue_3 (`|CreateWidget` "/Game/GrabAndInspect/BW_InspectionScreen.BW_InspectionScreen_C" null (`self.ItemDescription`)))
  (bind _output_get (set `self.InspectionUI` _returnvalue_3))
  (`UserWidget.AddToViewport` _output_get 0)
  (`self.DisableInput` (`self.Player`) _returnvalue)
  (`self.EnableInput` _returnvalue)
  (`self.K2_SetActorLocation` (+ (`PlayerCameraManager.GetCameraLocation` _returnvalue_2) (* (`KismetMathLibrary.GetForwardVector` (`PlayerCameraManager.GetCameraRotation` _returnvalue_2)) 200))))

(fn `StopInspecting`
  (`self.DisableInput` (`GameplayStatics.GetPlayerController` 0))
  (`Widget.SetVisibility` (`/Game/FirstPerson/Blueprints/BP_FirstPersonCharacter.HUD` (`self.Player`)) "Hidden")
  (`Widget.SetVisibility` (`self.InspectionUI`) "Hidden")
  (`self.EnableInput` (`self.Player`) null)
  (`self.K2_SetActorRelativeLocation` (0.0 0.0 0.0))
  (`self.K2_SetActorRelativeRotation` (struct)))

(fn `UserConstructionScript`)